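; BP_OfficeZPlayer is a player Blueprint that toggles the visibility of a Paper2D sprite.
; The sprite is hidden on BeginPlay, shown when another actor begins overlapping, and hidden when any overlap ends.
; Holding NumPad Two also shows the sprite, and releasing it hides the sprite regardless of overlap state.
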(event EventBeginPlay
  (Rendering|SetVisibility (Variables|Default|GetPaperSprite) false false))

(event Collision|EventActorEndOverlap
  (params (OtherActor :type Actor%20Object%20Reference))
  (Rendering|SetVisibility (Variables|Default|GetPaperSprite) false false))

(event EventTick
  (params (DeltaSeconds :type Float%20%28single-precision%29)))

(event Collision|EventActorBeginOverlap
  (params (OtherActor :type Actor%20Object%20Reference))
  (Rendering|SetVisibility (Variables|Default|GetPaperSprite) true false))

(event Input|KeyboardEvents|NumPadTwo
  (params (Key :type Key%20Structure :default "None"))
  (:Pressed
    (Rendering|SetVisibility (Variables|Default|GetPaperSprite) true false))
  (:Released
    (Rendering|SetVisibility (Variables|Default|GetPaperSprite) false false)))

(fn ConstructionScript)